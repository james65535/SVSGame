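; Gameplay ability that lets a spy interact with a target and open its inventory.
; On success, it takes the SpyCharacter and InteractInterface target from the event payload and calls Interact.
; If the target has an inventory, the SpyPlayerController displays it, then the ability ends; without one, it just ends.
; Failed character or interface casts cancel the ability, as does the failure event, which also logs.
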(event `self.InteractionSuccess`
  (params (Payload :type "GameplayEventData Structure"))
  (bind (_eventtag _instigator _target _optionalobject) (break `GameplayEventData` Payload))
  (bind _asspy_character (cast `SpyCharacter` _instigator)
    (:`then`
      (set `self.SpyCharacter` _asspy_character)
      (bind _asinteract_interface (cast `InteractInterface` _optionalobject)
        (:`then`
          (bind _output_get (set `self.TargetInteractionComponent` _asinteract_interface))
          (`InteractInterface.Interact` _output_get (`self.SpyCharacter`))
          (bind _returnvalue (`InteractInterface.HasInventory` (`self.TargetInteractionComponent`)))
          (if _returnvalue
            (bind _asspy_player_controller (cast `SpyPlayerController` (`Pawn.GetController` (`self.SpyCharacter`))))
            (bind _returnvalue_2 (`InteractInterface.GetInventory` (`self.TargetInteractionComponent`)))
            (`SpyPlayerController.C_DisplayTargetInventory` _asspy_player_controller _returnvalue_2)
            (`self.K2_EndAbility`)
            (else
              (`self.K2_EndAbility`))))
        (:`CastFailed`
          (`self.K2_CancelAbility` :!label _label))))
    (:`CastFailed`
      (goto _label))))

(event `self.InteractionFail`
  (params (Payload :type "GameplayEventData Structure"))
  (`KismetSystemLibrary.LogString` "Interact Ability Failed")
  (`self.K2_CancelAbility`))