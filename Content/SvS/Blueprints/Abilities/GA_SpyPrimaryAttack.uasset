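; Gameplay ability for the spy's primary attack, which plays an attack animation and applies damage when it hits.
; After committing, it waits on a custom task for a hit or no-hit gameplay event while the spy resets hit detection and animates.
; A hit applies the spy attack damage effect to the event's target data and ends; a miss cancels.
; OnEndAbility only logs leftover tasks; explicit task cleanup sits unconnected.
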(event `self.K2_ActivateAbility`
  (bind _returnvalue (`self.K2_CommitAbility`))
  (if _returnvalue
    (bind (_asynctaskproxy _payload) (`AbilityTaskSuccessFailEvent.WaitSuccessFailEvent` (struct :`TagName` "Attack.Hit") (struct :`TagName` "Attack.NoHit") null true true)
      (:`then`
        (set `self.AsyncTask` _asynctaskproxy)
        (bind _asspy_character (cast `SpyCharacter` (`.AvatarActor` (break `GameplayAbilityActorInfo` (`self.GetActorInfo`))))
          (:`then`
            (`SpyCharacter.ResetAttackHitFound` _asspy_character)
            (`SpyCharacter.PlayAttackAnimation` _asspy_character 0.3))
          (:`CastFailed`
            (`KismetSystemLibrary.LogString` "Cast to spy failed - cannot play attack animation")
            (`self.K2_CancelAbility`))))
      (:`SuccessEventReceived`
        (bind _output_get (set `self.Payload` _payload))
        (`self.BP_ApplyGameplayEffectToTarget` (`.TargetData` (break `GameplayEventData` _output_get)) "/Game/SvS/Blueprints/Abilities/GE_SpyAttackDamage.GE_SpyAttackDamage_C")
        (`self.K2_EndAbility`))
      (:`FailEventReceived`
        (`self.K2_CancelAbility`)))
    (else
      (`KismetSystemLibrary.LogString` "GA-PrimaryAttack Could not commit ability"))))

(event `self.K2_OnEndAbility`
  (params (bWasCancelled :type Boolean))
  ;[1 1 1] Should clean up its own tasks
  (`KismetSystemLibrary.LogString` (`KismetStringLibrary.Concat_StrStr` "GA-PrimaryAttack EndAbility was called and was cancelled: " (`KismetStringLibrary.Conv_BoolToString` bWasCancelled)))
  (bind _returnvalue (`self.AreTasksStillActive`))
  (if _returnvalue
    (`self.PrintActiveTaskNames`)
    (`KismetSystemLibrary.LogString` "GA-PrimaryAttack Called EndAbility but still has tasks")))