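; A static Gameplay Cue Notify that plays explosion feedback when a triggered trap impacts.
; On execute it spawns an explosion Niagara system at the target actor's location and a reduced-volume bomb sound attached to the target's root component.
; It also logs the target's network role, name and location alongside the cue parameters' location, which is not used for placing the effects.
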(fn `OnExecute`
  (params (MyTarget :type "Actor Object Reference") (Parameters :type "GameplayCueParameters Structure (by ref)"))
  (returns (ReturnValue :type Boolean))
  (bind _returnvalue (`Actor.K2_GetActorLocation` MyTarget))
  (`KismetSystemLibrary.LogString` (`KismetStringLibrary.Concat_StrStr` (`|GetEnumeratorNameAsString` (`Actor.GetLocalRole` MyTarget)) " Player: " (`KismetSystemLibrary.GetDisplayName` null) " Location: " (`KismetStringLibrary.Conv_VectorToString` _returnvalue)))
  (`KismetSystemLibrary.LogString` (`KismetStringLibrary.Concat_StrStr` "Paraneters location: " (`KismetStringLibrary.Conv_VectorToString` Parameters_Location)))
  (`NiagaraFunctionLibrary.SpawnSystemAtLocation` MyTarget "/Game/SvS/Blueprints/Niagara/FXS_ExplosionBlast.FXS_ExplosionBlast" _returnvalue)
  (`GameplayStatics.SpawnSoundAttached` "/Game/SvS/Assets/SoundCues/Weapons/SC_BombExplosion.SC_BombExplosion" (`Actor.RootComponent` MyTarget) "None" (0.0 0.0 0.0) (struct) "SnapToTarget" true 0.2 1.0 0.0 null null)
  (return false))