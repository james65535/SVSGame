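; Gameplay cue notify that plays the attack effects when an acid bath trap is triggered.
; On execute, it reads the trap asset from the cue's source object and spawns that asset's visual effect above the instigator's colliding bounds.
; The asset's attack sound attaches to the spawned effect, starts partway into the clip and stops when the effect is destroyed.
; An invalid trap asset or instigator is only logged.
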(fn `OnExecute`
  (params (MyTarget :type "Actor Object Reference") (Parameters :type "GameplayCueParameters Structure (by ref)"))
  (returns (ReturnValue :type Boolean))
  (locals (LocationOffset :type "Vector Structure" :default (0.0 0.0 100.0)) (TrapAsset :type "InventoryTrapAsset Object Reference"))
  (bind (_origin _boxextent) (`Actor.GetActorBounds` Parameters_Instigator true false))
  (bind _trapasset (`local.TrapAsset`))
  (bind _asinventory_trap_asset (cast `InventoryTrapAsset` Parameters_SourceObject)
    (:`then`
      (set `local.TrapAsset` _asinventory_trap_asset)
      (`/Engine/EditorBlueprintResources/StandardMacros.IsValid` Parameters_Instigator
        (:`Is Valid`
          (bind _returnvalue (`NiagaraFunctionLibrary.SpawnSystemAtLocation` Parameters_Instigator (`InventoryWeaponAsset.AttackVisualEffect` _trapasset) (+ _origin (`KismetMathLibrary.MakeVector` 0.0 0.0 (* (.z _boxextent) 1.2))) (struct :`Pitch` 180.0)))
          (`GameplayStatics.SpawnSoundAttached` (`InventoryWeaponAsset.AttackSoundEffect` _trapasset) _returnvalue "None" (0.0 0.0 0.0) (struct) "SnapToTarget" true 1.0 1.0 25.0 null null)
          (return false))
        (:`Is Not Valid`
          (`KismetSystemLibrary.LogString` "Acid Bath Causer is Invalid")
          (return false))))
    (:`CastFailed`
      (`KismetSystemLibrary.LogString` "Acid Bath has invalid trap asset")
      (return false))))