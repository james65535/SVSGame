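; GA_SpyTrapTrigger is a server-only gameplay ability for triggering traps on a spy character.
; ActivateAbility is empty: the commit, Hit/NoHit event wait and animation call are all disconnected.
; ProcessTrapTriggerSuccess, called only from that unwired chain, applies a gameplay effect to the owner and plays the cue from the payload's first target tag.
; OnEndAbility ends the stored task and logs cancellation and any lingering tasks.
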(event `self.K2_ActivateAbility`
  ;[1 0.1927 0.1927] Note this ability is server only
)

(event `self.K2_OnEndAbility`
  (params (bWasCancelled :type Boolean))
  ;[1 1 1] Task cleanup on end
  (bind _abilitytask (`self.AbilityTask`)
    (:`then`
      (`GameplayTask.EndTask` _abilitytask))
    (:`else`
      _))
  (`KismetSystemLibrary.LogString` (`KismetStringLibrary.Concat_StrStr` "GA-TrapTrigger EndAbility was called and was cancelled: " (`KismetStringLibrary.Conv_BoolToString` bWasCancelled)))
  (bind _returnvalue (`self.AreTasksStillActive`))
  (if _returnvalue
    (`self.PrintActiveTaskNames`)))

(fn `ProcessTrapTriggerSuccess`
  (params (InGameplayEventData :type "GameplayEventData Structure (by ref)"))
  (bind (_eventtag _instigator _target _optionalobject _optionalobject2 _contexthandle _instigatortags _targettags) (break `GameplayEventData` InGameplayEventData))
  (if (and (`BlueprintGameplayTagLibrary.MatchesTag` _eventtag (struct :`TagName` "TrapTrigger.Hit") true) (> (`BlueprintGameplayTagLibrary.GetNumGameplayTagsInContainer` _targettags) 0))
    (`self.BP_ApplyGameplayEffectToOwner` (`self.GameplayEffectClass`))
    ;[1 1 1] Presumes only 1 gameplaycue tag for triggering effects
    (`self.K2_ExecuteGameplayCue` (`|GetArrayItem` (`BlueprintGameplayTagLibrary.BreakGameplayTagContainer` _targettags)))
    (else
      (`self.K2_CancelAbility`))))